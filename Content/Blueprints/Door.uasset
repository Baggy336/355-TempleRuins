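; Interactive door that the first-person player swings open and that closes automatically when they leave.
; The Detect_Player volume enables Interact input on overlap, then disables it and reverses the timeline on exit.
; The timeline drives DoorMesh yaw up to MaxRotation, with play rate scaled from OpenSpeed over MaxRotation.
; Opening away from the player is unfinished: Open_Away does nothing and its dot-product direction check is disconnected.
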(event `Open_Away`
  ;[1 1 1] Trying to get the door to open away.
  (if (`self.isDoorClosed`)
    _))

(event `self.ReceiveBeginPlay`
  ;[1 1 1] Set the playrate of the door's animation.
  (`TimelineComponent.SetPlayRate` (`self.Open_Door`) (/ (`self.openSpeed`) (`self.MaxRotation`))))

(event `self.Detect_Player.OnComponentBeginOverlap`
  (params (OverlappedComponent :type "PrimitiveComponent Object Reference") (OtherActor :type "Actor Object Reference") (OtherComp :type "PrimitiveComponent Object Reference") (OtherBodyIndex :type Integer) (bFromSweep :type Boolean) (SweepResult :type "HitResult Structure (by ref)"))
  ;[1 1 1] Enable player interaction for the door's hitbox.
  (cast `/Game/Blueprints/FirstPersonCharacter` OtherActor)
  (`self.EnableInput` (`GameplayStatics.GetPlayerController` 0)))

(event `InputAction|Interact`
  (params (Key :type "Key Structure"))
  ;[1 1 1] Play the door_open animation on interaction.
  (:`Pressed`
    (bind (_direction _percent) (`Timeline|Open_Door` :!label _label)
      (:`Update`
        (`SceneComponent.K2_SetRelativeRotation` (`self.Door_Mesh`) (`KismetMathLibrary.MakeRotator` 0.0 0.0 (* _percent (`self.MaxRotation`))) false false)))))

(event `self.Detect_Player.OnComponentEndOverlap`
  (params (OverlappedComponent :type "PrimitiveComponent Object Reference") (OtherActor :type "Actor Object Reference") (OtherComp :type "PrimitiveComponent Object Reference") (OtherBodyIndex :type Integer))
  ;[1 1 1] Enable player interaction for the door's hitbox.
  (cast `/Game/Blueprints/FirstPersonCharacter` OtherActor)
  (`self.DisableInput` (`GameplayStatics.GetPlayerController` 0))
  (goto _label :!via `Reverse`))

(fn `UserConstructionScript`)