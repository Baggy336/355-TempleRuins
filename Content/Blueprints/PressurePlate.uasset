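; Pressure plate that controls a linked ToggleableObject when the first-person character steps on it.
; Collider overlaps play a timeline that lerps the moving piece down from its starting position, then reverse it on exit.
; Every timeline update, in either direction, sends TurnOn or TurnOff based on IsActive and PlayerisOn.
; Stepping off an active plate leaves PlayerisOn set, so the object keeps receiving TurnOn.
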(event `self.ReceiveBeginPlay`
  (bind (_returnvalue_location _returnvalue_rotation _returnvalue_scale) (`KismetMathLibrary.BreakTransform` (`SceneComponent.GetRelativeTransform` (`self.MovingPiece`))))
  ;[1 1 1] Set Out Position/In Position
  (set `self.StartingLocation ` (`KismetMathLibrary.MakeTransform` _returnvalue_location _returnvalue_rotation _returnvalue_scale))
  (set `self.EndingLocation` (`KismetMathLibrary.MakeTransform` (- _returnvalue_location (0.0 0.0 10.0)) _returnvalue_rotation _returnvalue_scale)))

(event `self.Collider.OnComponentBeginOverlap`
  (params (OverlappedComponent :type "PrimitiveComponent Object Reference") (OtherActor :type "Actor Object Reference") (OtherComp :type "PrimitiveComponent Object Reference") (OtherBodyIndex :type Integer) (bFromSweep :type Boolean) (SweepResult :type "HitResult Structure (by ref)"))
  (bind _controlledobject (`self.ControlledObject`))
  (bind _controlledobject_2 (`self.ControlledObject`))
  ;[1 1 1] When the player steps on the pressure plate, check if the controlled object is valid, and check for the state of the pressure plate.
  (cast `/Game/Blueprints/FirstPersonCharacter` OtherActor)
  (`/Engine/EditorBlueprintResources/StandardMacros.IsValid` _controlledobject
    (:`Is Valid`
      (if (`KismetSystemLibrary.DoesImplementInterface` _controlledobject "/Game/Blueprints/ToggleableObject.ToggleableObject_C")
        (if (`self.IsActive`)
          (set `self.PlayerisOn` true)
          ;[1 1 1] Play the animation
          (bind (_direction _press) (`Timeline|Animate_Press` :!label _label)
            (:`Update`
              (`SceneComponent.K2_SetRelativeTransform` (`self.MovingPiece`) (`KismetMathLibrary.TLerp` (`self.StartingLocation `) (`self.EndingLocation`) _press) false false)
              ;[1 1 1] Set the pressure plate's state and send a message to the object.
              (if (`self.IsActive`)
                (if (`self.PlayerisOn`)
                  (message `/Game/Blueprints/ToggleableObject.Turn On` _controlledobject_2)
                  (else
                    (message `/Game/Blueprints/ToggleableObject.Turn Off` _controlledobject_2 :!label _label_2)))
                (else
                  (set `self.PlayerisOn` false)
                  (goto _label_2)))))
          (else
            (goto _label)))))))

(event `self.Collider.OnComponentEndOverlap`
  (params (OverlappedComponent :type "PrimitiveComponent Object Reference") (OtherActor :type "Actor Object Reference") (OtherComp :type "PrimitiveComponent Object Reference") (OtherBodyIndex :type Integer))
  (bind _controlledobject (`self.ControlledObject`))
  ;[1 1 1] When the player steps on the pressure plate, check if the controlled object is valid, and check for the state of the pressure plate.
  (cast `/Game/Blueprints/FirstPersonCharacter` OtherActor)
  (`/Engine/EditorBlueprintResources/StandardMacros.IsValid` _controlledobject
    (:`Is Valid`
      (if (`KismetSystemLibrary.DoesImplementInterface` _controlledobject "/Game/Blueprints/ToggleableObject.ToggleableObject_C")
        (if (`self.IsActive`)
          (goto _label :!via `ReverseFromEnd`)
          (else
            (set `self.PlayerisOn` false)
            (goto _label :!via `ReverseFromEnd`)))))))

(fn `UserConstructionScript`)