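; Pilotable helicopter that the player boards by possession, destroying their character, and exits near the ground via a spawned first-person character.
; Input flags drive per-axis functions that accumulate "velocity" values on Tick, applied directly as Mover's relative location, so they act as positions.
; A timeline spins the propeller while possessed, and axis inputs control the look.
; SetYaw derives yaw from left/right flags but is never called.
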(event `InputAction|Helicopter Left`
  (params (Key :type "Key Structure"))
  (:`Pressed`
    (set `self.MoveLeft` true))
  (:`Released`
    (set `self.MoveLeft` false)))

(event `InputAction|Helicopter Right`
  (params (Key :type "Key Structure"))
  (:`Pressed`
    (set `self.MoveRight` true))
  (:`Released`
    (set `self.MoveRight` false)))

(event `InputAction|Helicopter Forward`
  (params (Key :type "Key Structure"))
  (:`Pressed`
    (set `self.MoveForwards` true))
  (:`Released`
    (set `self.MoveForwards` false)))

(event `InputAction|helicopter Backward`
  (params (Key :type "Key Structure"))
  (:`Pressed`
    (set `self.MoveBackwards` true))
  (:`Released`
    (set `self.MoveBackwards` false)))

(event `InputAction|Helicopter Descend`
  (params (Key :type "Key Structure"))
  (:`Pressed`
    (set `self.Landing` true))
  (:`Released`
    (set `self.Landing` false)))

(event `InputAction|Helicopter Lift`
  (params (Key :type "Key Structure"))
  (:`Pressed`
    (set `self.LiftOff` true))
  (:`Released`
    (set `self.LiftOff` false)))

(event `self.ReceiveTick`
  (params (DeltaSeconds :type "Float (single-precision)"))
  ;[1 1 1] Check for inputs to add to velocity every tick
  (`self.SetXVelocity` DeltaSeconds)
  (`self.SetYVelocity` DeltaSeconds)
  (`self.SetZVelocity` DeltaSeconds)
  ;[1 1 1] Move the helicopter every tick
  (`SceneComponent.K2_SetRelativeLocation` (`self.Mover`) (`KismetMathLibrary.MakeVector` (`self.XVelocity`) (`self.YVelocity`) (`self.ZVelocity`)) false false)
  (`SceneComponent.K2_SetRelativeRotation` (`self.Mover`) (`KismetMathLibrary.MakeRotator` 0.0 0.0 (`self.Yaw`)) false false)
  ;[1 1 1] While the player is possessing the object, rotate the propeller
  (if (`self.PlayerPossessed`)
    (bind (_direction _animatepropeller) (`Timeline|LoopPropellor` :!label _label)
      (:`Update`
        (`SceneComponent.K2_SetRelativeRotation` (`self.PropellerBase`) (`KismetMathLibrary.MakeRotator` 0.0 0.0 (* _animatepropeller 1080.0)) false false)))
    (else
      (goto _label :!via `Stop`))))

(event `InputAction|Interact`
  (params (Key :type "Key Structure"))
  (bind _returnvalue (`SceneComponent.K2_GetComponentToWorld` (`self.Pit`)))
  (bind (_returnvalue_x _returnvalue_y _returnvalue_z) (`KismetMathLibrary.BreakVector` (`SceneComponent.K2_GetComponentLocation` (`self.Pit`))))
  ;[1 1 1] When the player presses E, respawn the first person character if the object is close to the ground.
  (:`Pressed`
    (if (< _returnvalue_z (`self.DismountHeight`))
      (set `self.PlayerPossessed` false)
      (bind _returnvalue_2 (`|SpawnActorFromClass` "/Game/Blueprints/FirstPersonCharacter.FirstPersonCharacter_C" (`KismetMathLibrary.MakeTransform` (`KismetMathLibrary.MakeVector` (.x (.location _returnvalue)) (+ (.y (.location _returnvalue)) 80.0) (.z (.location _returnvalue))) (`KismetMathLibrary.MakeRotator` 0.0 0.0 (.yaw (.rotation _returnvalue)))) "Undefined" "OverrideRootScale" (`self.GetOwner`) null))
      (`Controller.Possess` (`self.GetController`) _returnvalue_2)
      (else
        (`KismetSystemLibrary.PrintString` "You may not exit the helicopter, it is too far off the ground!")))))

(event `/Game/Blueprints/Interfaces/PlayerInteractive.Player Wants to Interact`
  (params (Player :type "/Game/Blueprints/FirstPersonCharacter Object Reference"))
  ;[1 1 1] On press E, possess the object and destroy the player.
  (set `self.PlayerPossessed` true)
  (`Controller.Possess` (`self.GetController` Player) self)
  (`self.K2_DestroyActor` Player))

(event `InputAxis|TurnRate`
  (params (AxisValue :type "Float (single-precision)"))
  ;[1 1 1] Stick Look
  (`self.AddControllerYawInput` (* AxisValue (`self.BaseTurnRate`) (`GameplayStatics.GetWorldDeltaSeconds`))))

(event `InputAxis|Turn` :overrideparent false
  (params (AxisValue :type "Float (single-precision)"))
  ;[1 1 1] Mouse look
  (`self.AddControllerYawInput` AxisValue))

(event `InputAxis|LookUp` :overrideparent false
  (params (AxisValue :type "Float (single-precision)"))
  ;[1 1 1] Mouse look
  (`self.AddControllerPitchInput` AxisValue))

(event `InputAxis|LookUpRate`
  (params (AxisValue :type "Float (single-precision)"))
  ;[1 1 1] Stick Look
  (`self.AddControllerPitchInput` (* AxisValue (`self.BaseLookUpRate`) (`GameplayStatics.GetWorldDeltaSeconds`))))

(fn `SetXVelocity`
  (params (DeltaTime :type "Float (double-precision)"))
  (locals (XDir :type "Float (double-precision)"))
  (if (`self.MoveForwards`)
    (set `local.XDir` 1.0)
    (set `self.XVelocity` (+ (`self.XVelocity`) (* DeltaTime (`local.XDir`) (`self.AccelerationMult`))) :!label _label)
    (else
      (set `local.XDir` 0.0)
      (if (`self.MoveBackwards`)
        (set `local.XDir` -1.0)
        (goto _label)
        (else
          (set `local.XDir` 0.0))))))

(fn `SetYaw`
  (params (DeltaTime :type "Float (double-precision)"))
  (locals (Rot :type "Float (double-precision)") (YawMult :type "Float (double-precision)" :default 400.0))
  (if (`self.MoveLeft`)
    (set `local.Rot` 1.0)
    (else
      (set `local.Rot` 0.0)
      (if (`self.MoveRight`)
        (set `local.Rot` -1.0)
        (else
          (set `local.Rot` 0.0)))))
  (set `self.Yaw` (+ (`self.Yaw`) (* DeltaTime (`local.Rot`) (`local.YawMult`)))))

(fn `SetYVelocity`
  (params (DeltaTime :type "Float (double-precision)"))
  (locals (YDis :type "Float (double-precision)") (NewRoll :type "Float (double-precision)") (NewYaw :type "Float (double-precision)") (MinRoll :type "Float (double-precision)" :default -20.0) (MaxRoll :type "Float (double-precision)" :default 20.0))
  (if (`self.MoveLeft`)
    (set `local.YDis` -1.0)
    (set `self.YVelocity` (+ (`self.YVelocity`) (* DeltaTime (`local.YDis`) (`self.AccelerationMult`))) :!label _label)
    (else
      (set `local.YDis` 0.0)
      (if (`self.MoveRight`)
        (set `local.YDis` 1.0)
        (goto _label)
        (else
          (set `local.YDis` 0.0))))))

(fn `SetZVelocity`
  (params (DeltaTime :type "Float (double-precision)"))
  (locals (ZDir :type "Float (double-precision)") (NewPitch :type "Float (double-precision)") (MinPitch :type "Float (double-precision)" :default -20.0) (MaxPitch :type "Float (double-precision)" :default 10.0))
  (if (`self.LiftOff`)
    (set `local.ZDir` 1.0)
    (set `self.ZVelocity` (+ (`self.ZVelocity`) (* (`local.ZDir`) DeltaTime (`self.AccelerationMult`))) :!label _label)
    (else
      (set `local.ZDir` 0.0)
      (if (`self.Landing`)
        (set `local.ZDir` -1.0)
        (goto _label)
        (else
          (set `local.ZDir` 0.0))))))

(fn `UserConstructionScript`)