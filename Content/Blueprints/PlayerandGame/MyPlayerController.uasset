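; Player controller Blueprint that owns the game's HUD widget and keeps it fed with player data.
; On BeginPlay it caches the MyGameInstance, creates the HUD widget, adds it to the viewport and refreshes it.
; UpdateTheHUD passes the game instance's PlayerDetails to the widget.
; When the controller is destroyed, it removes the HUD from its parent.
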(event `self.ReceiveBeginPlay`
  (bind _asmy_game_instance (cast `/Game/Blueprints/PlayerandGame/MyGameInstance` (`GameplayStatics.GetGameInstance`)))
  (set `self.TheGameInstance` _asmy_game_instance)
  (bind _returnvalue (`|CreateWidget` "/Game/Blueprints/Gui/HUD.HUD_C"))
  (bind _output_get (set `self.TheHUD` _returnvalue))
  (`UserWidget.AddToViewport` _returnvalue 0)
  (`UserWidget.AddToViewport` _output_get 0)
  (`self.UpdateTheHUD`))

(event `self.ReceiveDestroyed`
  (bind _thehud (`self.TheHUD`))
  (`/Engine/EditorBlueprintResources/StandardMacros.IsValid` _thehud
    (:`Is Valid`
      (`Widget.RemoveFromParent` _thehud))))

(event `UpdateTheHUD`
  (bind _thehud (`self.TheHUD`))
  (`/Engine/EditorBlueprintResources/StandardMacros.IsValid` _thehud
    (:`Is Valid`
      (`/Game/Blueprints/Gui/HUD.UpdateHUD` _thehud (`/Game/Blueprints/PlayerandGame/MyGameInstance.PlayerDetails` (`self.TheGameInstance`))))))

(fn `UserConstructionScript`)