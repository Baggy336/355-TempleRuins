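; Rideable minecart pawn that carries its own spline track, which the player drives forward and backward.
; The construction script tiles spline mesh pieces along the spline, clamping tangents to avoid squishing.
; Each tick, input accelerates a clamped velocity, Euler integration advances the spline distance, and the Mover follows it.
; Boarding possesses the cart and destroys the player's pawn; exiting spawns and possesses a new FirstPersonCharacter at the camera.
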(event `InputAction|Minecart Forward`
  (params (Key :type "Key Structure"))
  (:`Pressed`
    (set `self.PlayerWantsToMoveForward` true))
  (:`Released`
    (set `self.PlayerWantsToMoveForward` false)))

(event `InputAction|Minecart Backward`
  (params (Key :type "Key Structure"))
  (:`Pressed`
    (set `self.PlayerWantsToMoveBackward` true))
  (:`Released`
    (set `self.PlayerWantsToMoveBackward` false)))

(event `self.ReceiveTick`
  (params (DeltaSeconds :type "Float (single-precision)"))
  (`self.Accelerate` DeltaSeconds)
  ;[1 1 1] Euler physics implementation
  (`self.Euler Step` DeltaSeconds)
  (`self.PositionCart`))

(event `InputAction|Interact`
  (params (Key :type "Key Structure"))
  (bind _returnvalue (`SceneComponent.K2_GetComponentToWorld` (`self.Camera`)))
  ;[1 1 1] Get out of minecart/repossess character
  (:`Pressed`
    (bind _returnvalue_2 (`|SpawnActorFromClass` "/Game/Blueprints/PlayerandGame/FirstPersonCharacter.FirstPersonCharacter_C" (`KismetMathLibrary.MakeTransform` (.location _returnvalue) (`KismetMathLibrary.MakeRotator` 0.0 0.0 (.yaw (.rotation _returnvalue)))) "Undefined" "OverrideRootScale" (`self.GetOwner`) null))
    (`Controller.Possess` (`self.GetController`) _returnvalue_2)))

(event `/Game/Blueprints/Interfaces/PlayerInteractive.Player Wants to Interact`
  (params (Player :type "/Game/Blueprints/PlayerandGame/FirstPersonCharacter Object Reference"))
  ;[1 1 1] Have the player controller possess the pawn.
  (`Controller.Possess` (`self.GetController` Player) self)
  (`self.K2_DestroyActor` Player))

(event `InputAxis|TurnRate`
  (params (AxisValue :type "Float (single-precision)"))
  ;[1 1 1] Stick Look
  (`self.AddControllerYawInput` (* AxisValue (`self.BaseTurnRate`) (`GameplayStatics.GetWorldDeltaSeconds`))))

(event `InputAxis|Turn` :overrideparent false
  (params (AxisValue :type "Float (single-precision)"))
  ;[1 1 1] Mouse look
  (`self.AddControllerYawInput` AxisValue))

(event `InputAxis|LookUp` :overrideparent false
  (params (AxisValue :type "Float (single-precision)"))
  ;[1 1 1] Mouse look
  (`self.AddControllerPitchInput` AxisValue))

(event `InputAxis|LookUpRate`
  (params (AxisValue :type "Float (single-precision)"))
  ;[1 1 1] Stick Look
  (`self.AddControllerPitchInput` (* AxisValue (`self.BaseLookUpRate`) (`GameplayStatics.GetWorldDeltaSeconds`))))

(fn `Accelerate`
  (params (DT :type "Float (double-precision)"))
  (locals (Dir :type "Float (double-precision)"))
  (if (`self.PlayerWantsToMoveForward`)
    (set `local.Dir` 1.0))
  (if (`self.PlayerWantsToMoveBackward`)
    (set `local.Dir` (- (`local.Dir`) 1.0)))
  ;[1 1 1] Velocity = clamp(velocity + dt*acc*dir, -max, max)
  (set `self.Velocity` (`KismetMathLibrary.FClamp` (+ (`self.Velocity`) (* (`local.Dir`) DT (`self.AccelerationMult`))) (* (`self.MaxVelocity`) -1.0) (`self.MaxVelocity`))))

(fn `Euler Step`
  (params (DT :type "Float (double-precision)"))
  ;[1 1 1] Position += velocity * DeltaTime
  (set `self.PositionOnSpline` (`KismetMathLibrary.FClamp` (+ (`self.PositionOnSpline`) (* (`self.Velocity`) DT)) 0.0 (`SplineComponent.GetSplineLength` (`self.Spline`)))))

(fn `PositionCart`
  (bind _spline (`self.Spline`))
  (bind _positiononspline (`self.PositionOnSpline`))
  (`SceneComponent.K2_SetRelativeLocationAndRotation` (`self.Mover`) (`SplineComponent.GetLocationAtDistanceAlongSpline` _spline _positiononspline "Local") (`SplineComponent.GetRotationAtDistanceAlongSpline` _spline _positiononspline "Local") false false))

(fn `UserConstructionScript`
  (bind _spline (`self.Spline`))
  (bind _spline_2 (`self.Spline`))
  (for _index (range (`KismetMathLibrary.FTrunc` (/ (`SplineComponent.GetSplineLength` (`self.Spline`)) (`self.LengthOfPiece`))))
    (bind _returnvalue (`AddComponent|NODE_AddSplineMeshComponent-0`))
    (bind _returnvalue_2 (* _index (`self.LengthOfPiece`)))
    (bind _returnvalue_3 (* (+ _index 1) (`self.LengthOfPiece`)))
    (`SplineMeshComponent.SetStartAndEnd` _returnvalue (`SplineComponent.GetLocationAtDistanceAlongSpline` _spline_2 _returnvalue_2 "Local") (`KismetMathLibrary.ClampVectorSize` (`SplineComponent.GetTangentAtDistanceAlongSpline` _spline_2 _returnvalue_2 "Local") 0.0 (`self.LengthOfPiece`)) (`SplineComponent.GetLocationAtDistanceAlongSpline` _spline _returnvalue_3 "Local") (`KismetMathLibrary.ClampVectorSize` (`SplineComponent.GetTangentAtDistanceAlongSpline` _spline _returnvalue_3 "Local") 0.0 (`self.LengthOfPiece`)) true))
  (`self.PositionCart`))