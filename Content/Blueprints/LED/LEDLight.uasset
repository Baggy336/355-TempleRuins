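; LED light Blueprint that switches between red, green and blue.
; The construction script creates a dynamic material instance on the cylinder mesh and applies the current state's color.
; Each Trigger event advances the state in a red, green, blue loop, then sets the "LED Color" material parameter to match.
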(event `/Game/Blueprints/Interfaces/Triggerable.Trigger`
  ;[1 1 1] On trigger, set the state of the LED based on it's current state.
  (set `self.CurrentState` (select `/Game/Blueprints/LED/LEDColor` (`self.CurrentState`) :`NewEnumerator0` "NewEnumerator1" :`NewEnumerator1` "NewEnumerator2" :`NewEnumerator2` "NewEnumerator0" :!type "/Game/Blueprints/LED/LEDColor Enum"))
  ;[1 1 1] Update the LED material
  (`self.UpdateMaterialColor`))

(fn `UpdateMaterialColor`
  (`MaterialInstanceDynamic.SetVectorParameterValue` (`self.LED Material`) "LED Color" (select `/Game/Blueprints/LED/LEDColor` (`self.CurrentState`) :`NewEnumerator0` (struct :`R` 0.932292 :`B` 0.016955 :`A` 1.0) :`NewEnumerator1` (struct :`G` 0.895833 :`B` 0.010981 :`A` 1.0) :`NewEnumerator2` (struct :`G` 0.009266 :`B` 1.0 :`A` 1.0) :!type "LinearColor Structure")))

(fn `UserConstructionScript`
  (bind _returnvalue (`PrimitiveComponent.CreateDynamicMaterialInstance` (`self.Cylinder`) 0 "/Game/Blueprints/LED/LEDMaterial.LEDMaterial" "None"))
  (set `self.LED Material` _returnvalue)
  (`self.UpdateMaterialColor`))