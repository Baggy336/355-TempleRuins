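; Elevator Blueprint that builds its own shaft for a configurable number of floors and moves a sliding floor up and down it.
; The construction script stacks instanced wall meshes per floor, leaving the front open at the bottom and the back open at the top.
; A timeline, rate-scaled by velocity over shaft height, raises the floor on Turnon and reverses on TurnOff.
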(event `self.ReceiveBeginPlay`
  ;[1 1 1] When the game begins, set how fast each elevator will move based on its height.
  (`TimelineComponent.SetPlayRate` (`self.Animate_Up`) (/ (`self.Elevator Velocity`) (`self.Max Height`))))

(event `/Game/Blueprints/Interfaces/ToggleableObject.Turn On`
  ;[1 1 1] When the player interacts, animate the elevator until the height is reached, or the player exits the collider
  (bind (_direction _percent) (`Timeline|Animate_Up` :!label _label)
    (:`Update`
      (`SceneComponent.K2_SetRelativeLocation` (`self.Sliding-Floor`) (`KismetMathLibrary.MakeVector` 0.0 0.0 (* _percent (`self.Max Height`))) false false))))

(event `/Game/Blueprints/Interfaces/ToggleableObject.Turn Off`
  ;[1 1 1] When the player interacts, animate the elevator until the height is reached, or the player exits the collider
  (goto _label :!via `Reverse`))

(fn `UserConstructionScript`
  (locals (`Current Floor` :type Integer) (`Current Z` :type "Float (double-precision)"))
  (set `self.Max Height` (* (`self.Max Floors`) 400.0))
  (for _index (range (+ (`self.Max Floors`) 1))
    (bind _output_get (set `local.Current Floor` _index))
    (set `local.Current Z` (* _output_get 400.0))
    ;[1 1 1] Right Wall
    (`InstancedStaticMeshComponent.AddInstance` (`self.WallInstanceMesh`) (`KismetMathLibrary.MakeTransform` (`KismetMathLibrary.MakeVector` -200.0 210.0 (`local.Current Z`))))
    ;[1 1 1] Left Wall
    (`InstancedStaticMeshComponent.AddInstance` (`self.WallInstanceMesh`) (`KismetMathLibrary.MakeTransform` (`KismetMathLibrary.MakeVector` -200.0 -210.0 (`local.Current Z`))))
    ;[1 1 1] Back Wall
    (if (!= (`local.Current Floor`) (`self.Max Floors`))
      (`InstancedStaticMeshComponent.AddInstance` (`self.WallInstanceMesh`) (`KismetMathLibrary.MakeTransform` (`KismetMathLibrary.MakeVector` 210.0 -200.0 (`local.Current Z`)) (struct :`Yaw` 90.0))))
    ;[1 1 1] Front Wall
    (if (!= (`local.Current Floor`) 0)
      (`InstancedStaticMeshComponent.AddInstance` (`self.WallInstanceMesh`) (`KismetMathLibrary.MakeTransform` (`KismetMathLibrary.MakeVector` -210.0 -200.0 (`local.Current Z`)) (struct :`Yaw` 90.0))))))