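; Interactable push button that sends toggle messages to a ControlledObject implementing the ToggleableObject interface.
; BeginPlay caches MovingButton's resting transform and a pressed one offset along Y.
; On interaction, the Press_Button timeline lerps the button inward, sending TurnOn or TurnOff per IsButtonOn on every update.
; ReversePress then eases it back, flipping IsButtonOn on every update rather than once on finish.
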(event `self.ReceiveBeginPlay`
  (bind (_returnvalue_location _returnvalue_rotation _returnvalue_scale) (`KismetMathLibrary.BreakTransform` (`SceneComponent.GetRelativeTransform` (`self.MovingButton`))))
  ;[1 1 1] Set in position/ out position
  (set `self.StartingLocation` (`KismetMathLibrary.MakeTransform` _returnvalue_location _returnvalue_rotation _returnvalue_scale))
  (set `self.EndingLocation` (`KismetMathLibrary.MakeTransform` (- _returnvalue_location (0.0 10.0 0.0)) _returnvalue_rotation _returnvalue_scale)))

(event `/Game/Blueprints/PlayerInteractive.Player Wants to Interact`
  (params (Player :type "/Game/Blueprints/FirstPersonCharacter Object Reference"))
  (bind _controlledobject (`self.ControlledObject`))
  (bind _controlledobject_2 (`self.ControlledObject`))
  (`/Engine/EditorBlueprintResources/StandardMacros.IsValid` _controlledobject
    (:`Is Valid`
      (if (`KismetSystemLibrary.DoesImplementInterface` _controlledobject "/Game/Blueprints/ToggleableObject.ToggleableObject_C")
        ;[1 1 1] Animate the Button
        (bind (_direction _animate_press) (`Timeline|Press_Button` :!via `PlayFromStart` :!label _label)
          (:`Update`
            (`SceneComponent.K2_SetRelativeTransform` (`self.MovingButton`) (`KismetMathLibrary.TLerp` (`self.StartingLocation`) (`self.EndingLocation`) _animate_press) false false)
            (if (`self.IsButtonOn`)
              (message `/Game/Blueprints/ToggleableObject.Turn Off` _controlledobject_2)
              (else
                (message `/Game/Blueprints/ToggleableObject.Turn On` _controlledobject_2))))
          (:`Finished`
            (bind (_direction_2 _animate_press_2) (`Timeline|ReversePress` :!via `ReverseFromEnd`)
              (:`Update`
                (`SceneComponent.K2_SetRelativeTransform` (`self.MovingButton`) (`KismetMathLibrary.TLerp` (`self.StartingLocation`) (`self.EndingLocation`) _animate_press_2) false false)
                (if (`self.IsButtonOn`)
                  (set `self.IsButtonOn` false)
                  (else
                    (set `self.IsButtonOn` true)))))))
        (else
          (goto _label :!via `ReverseFromEnd`))))))

(fn `UserConstructionScript`)